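; Zombie enemy that chases a BP_Character it sees or is hit by, using PawnSensing, Health and ToolUser components.
; Sight and hit events store that character's current location and set Chasing.
; While Chasing, Tick issues a simple AI move to that last known location; the flag is never cleared.
; On death it unequips its tool and destroys itself; the physics drop for the tool is disconnected.
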(event OnSeePawn(PawnSensing)
  (params (Pawn :type Pawn%20Object%20Reference))
  (Variables|Default|SetChaseTarget Pawn)
  (bind _asbp_character (Utilities|Casting|CastToBP_Character (Variables|Default|GetChaseTarget)))
  (Variables|Default|SetLastSeenTargetLocation (Transformation|GetActorLocation _asbp_character))
  (Variables|Default|SetChasing true))

(event OnHit(Health)
  (params (Damage :type Integer) (Instagator :type Actor%20Object%20Reference))
  (bind _output_get (Variables|Default|SetChaseTarget Instagator))
  (Development|PrintString (Utilities|GetDisplayName _output_get))
  (bind _asbp_character (Utilities|Casting|CastToBP_Character (Variables|Default|GetChaseTarget)))
  (Variables|Default|SetLastSeenTargetLocation (Transformation|GetActorLocation _asbp_character))
  (Variables|Default|SetChasing true))

(event OnDeath(Health)
  (params (Instagator :type Actor%20Object%20Reference))
  (Development|PrintString "I'm dead")
  (bind _returnvalue (Class|ToolUser|Unequip (Variables|Default|GetToolUser)))
  (Actor|DestroyActor))

(event EventBeginPlay)

(event Collision|EventActorBeginOverlap
  (params (OtherActor :type Actor%20Object%20Reference)))

(event EventTick
  (params (DeltaSeconds :type Float%20%28single-precision%29))
  (if (Variables|Default|GetChasing)
    (AI|Navigation|SimpleMovetoLocation (AI|GetAIController self) (Variables|Default|GetLastSeenTargetLocation))))

(fn ConstructionScript)