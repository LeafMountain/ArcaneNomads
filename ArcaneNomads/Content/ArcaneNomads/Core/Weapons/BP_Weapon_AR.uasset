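; Assault rifle weapon that fires a BP_Bullet projectile from its ShootOrigin when used.
; GetShootRotation traces from the player camera out to Range, then aims the muzzle at the impact point, or the trace end on a miss, so shots converge on the view center.
; OnUse spawns the bullet with player 0's pawn as owner and instigator, sets its InitialSpeed after spawning and plays an explosion sound.
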(event EventOnUse
  (bind _returnvalue (Game|Player|GetPlayerPawn 0))
  (bind _audio (Variables|Default|GetAudio))
  ;[1 1 1] Fire Bullet
  (bind _rotation (CallFunction|GetShootRotation))
  (bind _returnvalue_2 (Game|SpawnActorfromClass "/Game/ArcaneNomads/Core/Weapons/BP_Bullet.BP_Bullet_C" (Math|Transform|MakeTransform (Transformation|GetWorldLocation (Variables|Default|GetShootOrigin)) _rotation) "AlwaysSpawn" _returnvalue _returnvalue))
  (Variables|/Script/Engine.ProjectileMovementComponent|SetInitialSpeed (Variables|/Game/ArcaneNomads/Core/Weapons/BP_Bullet.BP_Bullet_C|GetProjectileMovement _returnvalue_2) 1e+03)
  (Audio|Components|Audio|SetSound _audio "/Game/StarterContent/Audio/Explosion01.Explosion01")
  (Audio|Components|Audio|Play _audio 0.0))

(fn ConstructionScript)

(fn GetShootRotation
  (bind _returnvalue (Game|GetPlayerCameraManager 0))
  (bind _returnvalue_2 (Transformation|GetActorLocation _returnvalue))
  (bind (_outhit _returnvalue_3) (Collision|LineTraceByChannel _returnvalue_2 (+ _returnvalue_2 (* (Transformation|GetActorForwardVector _returnvalue) (Variables|Default|GetRange))) "TraceTypeQuery1" false 0 "None"))
  (return (Math|Rotator|FindLookatRotation (Transformation|GetWorldLocation (Variables|Default|GetShootOrigin)) (Math|Vector|SelectVector (.ImpactPoint (Collision|BreakHitResult _outhit)) (.TraceEnd (Collision|BreakHitResult _outhit)) _returnvalue_3))))